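; ForceField_BP is a force field with a visible component and six directional collision pieces, switched on or off by an Active flag.
; Every Tick reapplies that flag, setting the visual's visibility and switching all six sides between query-and-physics and no collision.
; The construction script applies the Material and Scale variables to the visual component only, leaving the collision pieces untouched.
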(event EventBeginPlay)

(event Collision|EventActorBeginOverlap
  (params (OtherActor :type Actor%20Object%20Reference)))

(event EventTick
  (params (DeltaSeconds :type Float%20%28single-precision%29))
  (bind _front (Variables|Default|Getfront))
  (bind _bottom (Variables|Default|GetBottom))
  (bind _active (Variables|Default|GetActive))
  (bind _top (Variables|Default|GetTop))
  (bind _right (Variables|Default|GetRight))
  (bind _left (Variables|Default|Getleft))
  (bind _back (Variables|Default|Getback))
  (Rendering|SetVisibility (Variables|Default|Geterrwerr) _active false)
  (if _active
    (Collision|SetCollisionEnabled _bottom "QueryAndPhysics")
    (Collision|SetCollisionEnabled _top "QueryAndPhysics")
    (Collision|SetCollisionEnabled _right "QueryAndPhysics")
    (Collision|SetCollisionEnabled _left "QueryAndPhysics")
    (Collision|SetCollisionEnabled _back "QueryAndPhysics")
    (Collision|SetCollisionEnabled _front "QueryAndPhysics")
    (else
      (Collision|SetCollisionEnabled _bottom "NoCollision")
      (Collision|SetCollisionEnabled _top "NoCollision")
      (Collision|SetCollisionEnabled _right "NoCollision")
      (Collision|SetCollisionEnabled _left "NoCollision")
      (Collision|SetCollisionEnabled _back "NoCollision")
      (Collision|SetCollisionEnabled _front "NoCollision"))))

(fn ConstructionScript
  (Rendering|Material|SetMaterial (Variables|Default|Geterrwerr) 0 (Variables|Default|GetMaterial))
  (Transformation|SetRelativeScale3D (Variables|Default|Geterrwerr) (Variables|Default|GetScale)))