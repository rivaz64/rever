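; Lever Blueprint that toggles an Active state on Press and drives two force fields with it.
; Tick sets ForceFieldActivar to the lever's state and ForceFieldDesactivar to its inverse.
; While Normal is true it records Active into the Estados array each frame; otherwise it steps backward through that history, rewinding the lever.
; Press also sets Normal back to true.
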(event EventBeginPlay
  (Input|EnableInput (Game|GetPlayerController 0)))

(event Collision|EventActorBeginOverlap
  (params (OtherActor :type Actor%20Object%20Reference)))

(event EventTick
  (params (DeltaSeconds :type Float%20%28single-precision%29))
  (Variables|/Game/Procedural/ForceField/ForceField_BP.ForceField_BP_C|SetActive (Variables|Default|GetForceFieldDesactivar) (not (Variables|Default|GetActive)))
  (Variables|/Game/Procedural/ForceField/ForceField_BP.ForceField_BP_C|SetActive (Variables|Default|GetForceFieldActivar) (Variables|Default|GetActive))
  (if (Variables|Default|GetNormal)
    (bind _returnvalue (Utilities|Array|Add (Variables|Default|GetEstados) (Variables|Default|GetActive)))
    (Variables|Default|SetEstadosIndex _returnvalue)
    (elif (> (Variables|Default|GetEstadosIndex) 0)
      (Variables|Default|SetActive (Utilities|Array|Get(acopy) (Variables|Default|GetEstados) (Variables|Default|GetEstadosIndex)))
      (Math|Integer|DecrementInt (Variables|Default|GetEstadosIndex)))))

(fn ConstructionScript)

(fn Press
  (Variables|Default|SetActive (not (Variables|Default|GetActive)))
  (Variables|Default|SetNormal true)
  (Development|PrintString "Hello"))